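; BP_Test is a test pawn that uses AI movement to travel between BP_Only_TargetPoint actors in the level.
; BeginPlay collects the points, and Tick accumulates time, repeatedly calling AIMoveTo toward the current point once a three-second delay passes.
; On success, an Arrive flag gates resetting the timer and advancing the wrapping index.
; Arrive is cleared there and never set back to true in this graph.
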(event `self.ReceiveBeginPlay`
  (bind _outactors (`GameplayStatics.GetAllActorsOfClass` "/Game/Wise/Blueprints/BP_Only_TargetPoint.BP_Only_TargetPoint_C"))
  (set `self.Target Point` _outactors))

(event `self.ReceiveTick`
  (params (DeltaSeconds :type "Float (single-precision)"))
  (set `self.DelayTime` (+ DeltaSeconds (`self.DelayTime`)))
  (if (> (`self.DelayTime`) 3.0)
    (`|AIMoveTo` self (0.0 0.0 0.0) (`|GetArrayItem` (`self.Target Point`) (`self.Target Array`))
      (:`OnSuccess`
        (if (`self.Arrive`)
          (set `self.Arrive` false)
          (set `self.DelayTime` 0.0)
          (if (== (+ (`self.Target Array`) 1) (`KismetArrayLibrary.Array_Length` (`self.Target Point`)))
            (set `self.Target Array` 0)
            (else
              (`/Engine/EditorBlueprintResources/StandardMacros.IncrementInt` (`self.Target Array`)))))))))

(fn `UserConstructionScript`)